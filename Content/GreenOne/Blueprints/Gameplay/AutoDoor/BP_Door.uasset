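; BP_Door is an automatic door that slides a Cube vertically when a BP_Player enters its Box trigger.
; The Move timeline offsets the Cube's relative Z from the location cached at BeginPlay, and reverses when the player leaves.
; Each timeline update sets Finish while the offset is below a threshold; entering plays the timeline if Finish is true, otherwise reverses it.
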(event `self.ReceiveBeginPlay`
  (set `self.Relative Location` (`SceneComponent.RelativeLocation` (`self.Cube`))))

(event `self.Box.OnComponentBeginOverlap`
  (params (OverlappedComponent :type "PrimitiveComponent Object Reference") (OtherActor :type "Actor Object Reference") (OtherComp :type "PrimitiveComponent Object Reference") (OtherBodyIndex :type Integer) (bFromSweep :type Boolean) (SweepResult :type "HitResult Structure (by ref)"))
  (cast `/Game/GreenOne/Blueprints/BP_Player` OtherActor)
  (if (`self.Finish`)
    (bind (_direction _move) (`Timeline|Move` :!label _label)
      (:`Update`
        (`SceneComponent.K2_SetRelativeLocation` (`self.Cube`) (`KismetMathLibrary.MakeVector` (.x (`self.Relative Location`)) (.y (`self.Relative Location`)) (+ _move (.z (`self.Relative Location`)))) false false)
        (set `self.Finish` (< _move 700.0))))
    (else
      (goto _label :!via `Reverse`))))

(event `self.Box.OnComponentEndOverlap`
  (params (OverlappedComponent :type "PrimitiveComponent Object Reference") (OtherActor :type "Actor Object Reference") (OtherComp :type "PrimitiveComponent Object Reference") (OtherBodyIndex :type Integer))
  (cast `/Game/GreenOne/Blueprints/BP_Player` OtherActor)
  (goto _label :!via `Reverse`))

(fn `UserConstructionScript`)