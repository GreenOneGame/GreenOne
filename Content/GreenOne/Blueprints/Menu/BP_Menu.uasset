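; BP_Menu drives the main menu scene, creating the UI_MainMenu widget and pairing it with camera views for menu and options.
; On BeginPlay it shows the widget with mouse cursor and Game-and-UI input, then cuts to the menu camera.
; The widget's GoMenu and GoOption events are bound for navigation, with transition events blending between the two cameras.
; The first key press calls StartCredits on that same widget, stored as Credits.
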(event `Key|AnyKey`
  (params (Key :type "Key Structure"))
  (:`Pressed`
    (`/Engine/EditorBlueprintResources/StandardMacros.DoOnce` false
      (:`Completed`
        (`/Game/GreenOne/Widget/UI_MainMenu.StartCredits` (`self.Credits`))))))

(event `self.ReceiveBeginPlay`
  (bind _returnvalue (`GameplayStatics.GetPlayerController` 0))
  (bind _returnvalue_2 (`|CreateWidget` "/Game/GreenOne/Widget/UI_MainMenu.UI_MainMenu_C"))
  (bind _output_get (set `self.Credits` _returnvalue_2))
  (`UserWidget.AddToViewport` _returnvalue_2 0)
  (`WidgetBlueprintLibrary.SetInputMode_GameAndUIEx` _returnvalue _output_get)
  (set `PlayerController.bShowMouseCursor` true _returnvalue)
  (add `/Game/GreenOne/Widget/UI_MainMenu.OnGoMenu` _returnvalue_2 (`|CreateDelegate` :!event `TransitionMenu`))
  (add `/Game/GreenOne/Widget/UI_MainMenu.OnGoOption` _returnvalue_2 (`|CreateDelegate` :!event `TransitionOption`))
  (bind _cameramenu (`self.CameraMenu`)
    (:`then`
      (`PlayerController.SetViewTargetWithBlend` (`GameplayStatics.GetPlayerController` 0) _cameramenu 0.0 "VTBlend_Linear" 0.0 true))
    (:`else`)))

(event `TransitionMenu`
  (bind _cameramenu (`self.CameraMenu`)
    (:`then`
      (`PlayerController.SetViewTargetWithBlend` (`GameplayStatics.GetPlayerController` 0) _cameramenu 0.7 "VTBlend_Linear" 0.0 true))
    (:`else`)))

(event `TransitionOption`
  (bind _cameraoption (`self.CameraOption`)
    (:`then`
      (`PlayerController.SetViewTargetWithBlend` (`GameplayStatics.GetPlayerController` 0) _cameraoption 0.7 "VTBlend_Linear" 0.0 true))
    (:`else`)))

(fn `UserConstructionScript`)