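; Debug HUD Blueprint that draws a four-armed crosshair at the center of the screen.
; On each DrawHUD it draws four rectangles, left, right, above and below the screen's midpoint.
; Color, arm length, thickness and center gap come from variables, so the crosshair shape is adjustable without changing the graph.
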(event `self.ReceiveDrawHUD`
  (params (SizeX :type Integer) (SizeY :type Integer))
  (bind _crosslenght (`self.CrossLenght`))
  (bind _crossthickness (`self.CrossThickness`))
  (bind _crosslenght_2 (`self.CrossLenght`))
  (bind _crossthickness_2 (`self.CrossThickness`))
  (bind _crossthickness_3 (`self.CrossThickness`))
  (bind _crossthickness_4 (`self.CrossThickness`))
  (`self.DrawRect` (`self.CrossColor`) (- (`KismetMathLibrary.Conv_IntToDouble` (/ SizeX 2)) (+ _crosslenght_2 (`self.CrossSpacing`))) (- (`KismetMathLibrary.Conv_IntToDouble` (/ SizeY 2)) (/ _crossthickness 2.0)) _crosslenght_2 _crossthickness)
  (`self.DrawRect` (`self.CrossColor`) (+ (`KismetMathLibrary.Conv_IntToDouble` (/ SizeX 2)) (`self.CrossSpacing`)) (- (`KismetMathLibrary.Conv_IntToDouble` (/ SizeY 2)) (/ _crossthickness_2 2.0)) (`self.CrossLenght`) _crossthickness_2)
  (`self.DrawRect` (`self.CrossColor`) (- (`KismetMathLibrary.Conv_IntToDouble` (/ SizeX 2)) (/ _crossthickness_4 2.0)) (- (`KismetMathLibrary.Conv_IntToDouble` (/ SizeY 2)) (+ _crosslenght (`self.CrossSpacing`))) _crossthickness_4 _crosslenght)
  (`self.DrawRect` (`self.CrossColor`) (- (`KismetMathLibrary.Conv_IntToDouble` (/ SizeX 2)) (/ _crossthickness_3 2.0)) (+ (`KismetMathLibrary.Conv_IntToDouble` (/ SizeY 2)) (`self.CrossSpacing`)) _crossthickness_3 (`self.CrossLenght`)))

(fn `UserConstructionScript`)